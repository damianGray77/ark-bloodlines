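; Manager actor for the ArkBloodlines scanner that backfills the scanner buff onto tamed dinos near players.
; A looping timer started on BeginPlay periodically loops over all player controllers and gathers tames within a wide radius of each controlled pawn.
; Any tame lacking Buff_ArkBloodlineScanner receives it through StaticAddBuff.
; BeginPlay also caches the ShowDebugJson option from the game mode's INI settings.
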(event `self.ReceiveBeginPlay`
  (`|ExecutionSequence`
    (:`then_0`
      (`KismetSystemLibrary.K2_SetTimer` self "BackfillNearbyTames" 10.0 true false 5.0))
    (:`then_1`
      (bind _asshooter_game_mode (cast `ShooterGameMode` (`GameplayStatics.GetGameMode` null)))
      (bind _returnvalue (`ShooterGameMode.GetBoolOptionIni` _asshooter_game_mode "ArkBloodlinesScanner" "ShowDebugJson" false))
      (set `self.ShowDebugJson` _returnvalue false))))

(fn `BackfillNearbyTames`
  (bind _outactors (`GameplayStatics.GetAllActorsOfClass` null "/Script/ShooterGame.ShooterPlayerController"))
  (for _array_element _outactors
    (bind _asshooter_player_controller (cast `ShooterPlayerController` _array_element))
    (bind _dinos (`ShooterPlayerController.GetTamedDinosNearBy` _asshooter_player_controller 50000.0 (`self.K2_GetActorLocation` (`Controller.K2_GetPawn` _asshooter_player_controller))))
    (for _array_element_2 _dinos
      (if (not (`PrimalCharacter.HasBuff` _array_element_2 "/ArkBloodlinesScanner/Buff_ArkBloodlineScanner.Buff_ArkBloodlineScanner_C" false))
        (`PrimalBuff.StaticAddBuff` "/ArkBloodlinesScanner/Buff_ArkBloodlineScanner.Buff_ArkBloodlineScanner_C" _array_element_2 null null)))))

(fn `UserConstructionScript`)